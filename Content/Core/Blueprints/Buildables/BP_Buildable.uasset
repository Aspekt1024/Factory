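; BP_Buildable is a placeable build actor that can be moved, rotated, finalised or cancelled.
; Placement updates snap its location to a grid at the camera trace hit, and rotation input turns it in 45-degree yaw steps.
; Progressing immediately finalises, restoring the default material on child meshes and clearing the move timer, while cancelling destroys the actor.
; InitialiseBuild is empty here, and the hologram material instance is created but never applied.
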(event `self.ReceiveBeginPlay`
  (`self.InitialiseBuild`))

(event `UpdateBuildPos`
  (`self.UpdateLocation`))

(fn `CancelBuild`
  (returns (isComplete :type Boolean))
  (`self.K2_DestroyActor`)
  (return true))

(fn `FinaliseBuild`
  (bind _movebuildtimer (`self.moveBuildTimer`))
  (`self.SetAllMaterials` null true)
  (if (`KismetSystemLibrary.K2_IsValidTimerHandle` _movebuildtimer)
    (`KismetSystemLibrary.K2_ClearAndInvalidateTimerHandle` _movebuildtimer)
    (set `self.moveBuildTimer` (struct))))

(fn `InitialiseBuild`)

(fn `ProgressBuild`
  (returns (isComplete :type Boolean))
  (`self.FinaliseBuild`)
  (return true))

(fn `RotateBuild`
  (params (rotationInput :type "Float (double-precision)"))
  (`self.K2_SetActorRotation` (`KismetMathLibrary.MakeRotator` (.roll (`self.K2_GetActorRotation`)) (.pitch (`self.K2_GetActorRotation`)) (+ (.yaw (`self.K2_GetActorRotation`)) (* (`local.rotationInput`) 45.0)))))

(fn `SetAllMaterials`
  (params (materialOverride :type "MaterialInterface Object Reference") (useDefault :type Boolean))
  (for _array_element (`SceneComponent.GetChildrenComponents` (`self.DefaultSceneRoot`) false)
    (bind _asstatic_mesh_component (cast `StaticMeshComponent` _array_element))
    (for _index (range (`PrimitiveComponent.GetNumMaterials` _asstatic_mesh_component))
      (`PrimitiveComponent.SetMaterial` _asstatic_mesh_component _index (select `bool` (`local.useDefault`) :`false` (`local.materialOverride`) :`true` "/Engine/EngineMaterials/DefaultMaterial.DefaultMaterial")))))

(fn `UpdateLocation`
  (bind (_hitresult_out _ishit_out) (`PlayerSubsystem.LineTraceFromCamera` (subsystem `PlayerSubsystem`) "ECC_Visibility"))
  (if _ishit_out
    (`self.K2_SetActorLocation` (`KismetMathLibrary.Vector_SnappedToGrid` (`.ImpactPoint` (`GameplayStatics.BreakHitResult` _hitresult_out)) 50.0))))

(fn `UserConstructionScript`
  (bind _returnvalue (`KismetMaterialLibrary.CreateDynamicMaterialInstance` "/Game/Core/Assets/Materials/MI_Hologram.MI_Hologram"))
  (set `self.MI_Hologram` _returnvalue))