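; Buildable conveyor support with adjustable height, previewed with a hologram material and placed in two stages.
; The first confirm locks location, then player look height sets a clamped, grid-snapped height; cancel steps back to positioning.
; Height changes rebuild instanced middle segments and move the top mesh, or show a single standard mesh at zero.
; Finalising enables collision and spawns a BP_AttachPoint actor at the attach point.
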(event `self.UpdateBuildPos`
  (if (`self.isLocationLocked`)
    ;[0.01447 0.1467 0.1962] Update Height
    (set `self.HeightOverride` (`KismetMathLibrary.FClamp` (`KismetMathLibrary.GridSnap_Float` (`PlayerSubsystem.GetLookHeightAboveObject` (subsystem `PlayerSubsystem`) self) 50.0) 0.0 200.0))
    (`self.UpdateMeshHeight`)
    (else
      ;[0.01447 0.1467 0.1962] Update Location
      (`self.UpdateLocation`))))

(fn `CancelBuild`
  (returns (isComplete :type Boolean))
  (if (`self.isLocationLocked`)
    (set `self.isLocationLocked` false)
    (set `self.HeightOverride` 0.0)
    (`self.UpdateMeshHeight`)
    (return false)
    (else
      (bind _iscomplete (`parent.CancelBuild`))
      (return _iscomplete))))

(fn `FinaliseBuild`
  (`PrimitiveComponent.SetCollisionEnabled` (`self.Top`) "QueryAndPhysics")
  (`PrimitiveComponent.SetCollisionEnabled` (`self.ISM_Mid`) "QueryAndPhysics")
  (`PrimitiveComponent.SetCollisionEnabled` (`self.Base`) "QueryAndPhysics")
  (bind _returnvalue (`|SpawnActorFromClass` "/Game/Core/Blueprints/Buildables/BP_AttachPoint.BP_AttachPoint_C" (`SceneComponent.K2_GetComponentToWorld` (`self.AttachPoint`)) "Undefined" "MultiplyWithRoot" null null))
  (set `self.AttachBP` _returnvalue)
  (`parent.FinaliseBuild`))

(fn `InitialiseBuild`
  (`parent.InitialiseBuild`)
  (`self.UpdateMeshHeight`))

(fn `ProgressBuild`
  (params (overrideCompletion :type Boolean))
  (returns (isComplete :type Boolean))
  (if (`self.isLocationLocked`)
    (if (not overrideCompletion)
      (`self.FinaliseBuild`))
    (return true)
    (else
      (set `self.isLocationLocked` true)
      (`self.OnLocationLocked`)
      (return false))))

(fn `UpdateMeshHeight`
  (`InstancedStaticMeshComponent.ClearInstances` (`self.ISM_Mid`))
  (if (== (`self.HeightOverride`) 0.0)
    (`SceneComponent.K2_SetRelativeLocation` (`self.Top`) (0.0 0.0 0.0) false false)
    (`SceneComponent.SetHiddenInGame` (`self.Base`) true false)
    (`SceneComponent.SetHiddenInGame` (`self.ISM_Mid`) true false)
    (`StaticMeshComponent.SetStaticMesh` (`self.Top`) "/Game/Core/Assets/ConveyorSupportStandard.ConveyorSupportStandard")
    (else
      (`SceneComponent.SetHiddenInGame` (`self.Base`) false false)
      (`SceneComponent.SetHiddenInGame` (`self.ISM_Mid`) false false)
      (for _index (range (`KismetMathLibrary.FTrunc` (/ (`self.HeightOverride`) 50.0)))
        (switch `int` _index
          (:`Default`
            (`InstancedStaticMeshComponent.AddInstance` (`self.ISM_Mid`) (`KismetMathLibrary.MakeTransform` (* _index (0.0 0.0 50.0))) false))))
      (`StaticMeshComponent.SetStaticMesh` (`self.Top`) "/Game/Core/Assets/ConveyorSupportTop.ConveyorSupportTop")
      (`SceneComponent.K2_SetRelativeLocation` (`self.Top`) (* (`self.HeightOverride`) (0.0 0.0 1.0)) false false))))

(fn `UserConstructionScript`
  (`parent.UserConstructionScript`)
  (`PrimitiveComponent.SetMaterial` (`self.Base`) 0 (`self.MI_Hologram`))
  (`PrimitiveComponent.SetMaterial` (`self.Top`) 0 (`self.MI_Hologram`))
  (`PrimitiveComponent.SetMaterial` (`self.ISM_Mid`) 0 (`self.MI_Hologram`)))