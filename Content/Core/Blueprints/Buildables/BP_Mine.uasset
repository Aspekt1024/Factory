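; BP_Mine is a buildable mine that produces items on a timer and hands them to the connected attach point.
; It creates an output attach point, whose connection is disabled when an attachment is added and re-enabled when all are removed.
; Each looping timer tick raises a capped item count, then spawns one item actor if the next attach point is valid.
; The file never decrements that count.
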(event `self.ReceiveBeginPlay`
  (`parent.ReceiveBeginPlay`)
  (bind _attachpoint (`self.Create AttachPoint` (`SceneComponent.K2_GetComponentToWorld` (`self.AttachPosition`))))
  (bind _output_get (set `self.AttachPoint` _attachpoint))
  (`AttachPoint.SetDirection` _output_get "Output")
  (bind _returnvalue (`KismetSystemLibrary.K2_SetTimerDelegate` (delegate `ProdutionEvent`) (`self.ProductionInterval`) true))
  (set `self.ProductionTimer` _returnvalue))

(event `ProdutionEvent`
  (`self.ProduceItems`))

(event `self.OnAttachmentAdded`
  (params (AttachPoint :type "AttachPoint Object Reference") (Other :type "AttachPoint Object Reference"))
  (`AttachPoint.SetConnectionEnabled` AttachPoint false))

(event `self.OnAllAttachmentsRemoved`
  (params (AttachPoint :type "AttachPoint Object Reference"))
  (`AttachPoint.SetConnectionEnabled` AttachPoint true))

(event `self.ReceiveAsyncPhysicsTick`
  (params (DeltaSeconds :type "Float (single-precision)") (SimSeconds :type "Float (single-precision)")))

(fn `CreateNewItem`
  (returns (item :type "/Game/Core/Blueprints/Items/BP_Item Object Reference"))
  (bind _returnvalue (`|SpawnActorFromClass` (`self.ItemType`) (`SceneComponent.K2_GetComponentToWorld` (`self.ItemEndPosition`)) "Undefined" "MultiplyWithRoot" null null))
  (return _returnvalue))

(fn `InitialiseBuild`
  (bind _attachpoint (`self.Create AttachPoint` (`SceneComponent.K2_GetComponentToWorld` (`self.AttachPosition`))))
  (set `self.AttachPoint` _attachpoint))

(fn `ProduceItems`
  (bind _nextattachpoint (`AttachPoint.NextAttachPoint` (`self.AttachPoint`)))
  (`|ExecutionSequence`
    (:`then_0`
      (set `self.ItemCount` (`KismetMathLibrary.Clamp` (+ (`self.ItemCount`) (`self.ProductionQuantity`)) 0 (`self.MaxItemCount`))))
    (:`then_1`
      (if (> (`self.ItemCount`) 0)
        (`/Engine/EditorBlueprintResources/StandardMacros.IsValid` _nextattachpoint
          (:`Is Valid`
            (bind _item (`self.CreateNewItem`))
            (`AttachPoint.GiveItem` _nextattachpoint _item)))))))

(fn `UserConstructionScript`
  (`parent.UserConstructionScript`))