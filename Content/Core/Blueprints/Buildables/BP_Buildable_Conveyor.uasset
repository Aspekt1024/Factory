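; Buildable conveyor belt placed in two stages, a start support and then an end support, with a hologram preview until placed.
; Placement, rotation and building forward to whichever support is active.
; Locking the start spawns the end support and initialises BuildableSpline between both attach points, then refreshes it as the end moves.
; New spline meshes get hologram materials, swapped on placement for default and dynamic belt materials.
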(event `OnBuildCreation`
  (add `BuildableSplineComponent.OnMeshComponentCreated` (`self.BuildableSpline`) (delegate `SplineMeshComponentCreated`)))

(event `SplineMeshComponentCreated`
  (params (SplineMeshComponent :type "SplineMeshComponent Object Reference"))
  (`PrimitiveComponent.SetMaterial` SplineMeshComponent 0 "/Game/Core/Assets/Materials/MI_Hologram.MI_Hologram")
  (`PrimitiveComponent.SetMaterial` SplineMeshComponent 1 "/Game/Core/Assets/Materials/MI_Hologram.MI_Hologram"))

(event `self.UpdateBuildPos`
  (bind _startsupport (`self.startSupport`))
  (bind (_returnvalue_location _returnvalue_rotation) (`KismetMathLibrary.BreakTransform` (`SceneComponent.K2_GetComponentToWorld` (`/Game/Core/Blueprints/Buildables/BP_Buildable_ConveyorSupport.AttachPoint` _startsupport))))
  (if (`self.isStartLocked`)
    (`self.UpdateBuildPos` (`self.endSupport`))
    (`BuildableSplineComponent.UpdateSpline` (`self.BuildableSpline`))
    (else
      (`self.UpdateBuildPos` _startsupport)
      (`self.K2_SetActorLocationAndRotation` _returnvalue_location _returnvalue_rotation))))

(fn `Build`
  (returns (isComplete :type Boolean))
  (if (`self.isStartLocked`)
    ;[0.01447 0.1467 0.1962] Build End Point
    (bind _iscomplete (`self.Build` (`self.endSupport`)))
    (if _iscomplete
      (`self.PlaceBuild`)
      (return true)
      (else
        (return false)))
    (else
      ;[0.01447 0.1467 0.1962] Build Start Point
      (bind _iscomplete_2 (`self.Build` (`self.startSupport`)))
      (bind _output_get (set `self.isStartLocked` _iscomplete_2))
      (if _output_get
        (bind _returnvalue (`|SpawnActorFromClass` "/Game/Core/Blueprints/Buildables/BP_Buildable_ConveyorSupport.BP_Buildable_ConveyorSupport_C" (`self.GetTransform`) "Undefined" "MultiplyWithRoot" null null))
        (set `self.endSupport` _returnvalue)
        (`ActorComponent.K2_DestroyComponent` (`self.Temp_Conveyor`))
        (`self.SetAllMaterials` (`self.MI_Hologram`))
        (`BuildableSplineComponent.InitialiseSpline` (`self.BuildableSpline`) (`self.Spline`) (`/Game/Core/Blueprints/Buildables/BP_Buildable_ConveyorSupport.AttachPoint` (`self.startSupport`)) (`/Game/Core/Blueprints/Buildables/BP_Buildable_ConveyorSupport.AttachPoint` (`self.endSupport`)))
        (return false)
        (else
          (return false))))))

(fn `CreateBuild`
  (`parent.CreateBuild`)
  (bind _returnvalue (`|SpawnActorFromClass` "/Game/Core/Blueprints/Buildables/BP_Buildable_ConveyorSupport.BP_Buildable_ConveyorSupport_C" (`self.GetTransform`) "Undefined" "MultiplyWithRoot" null null))
  (set `self.startSupport` _returnvalue)
  (`self.SetAllMaterials` (`self.MI_Hologram`))
  (`self.OnBuildCreation`))

(fn `GetPosAndTangent`
  (params (index :type Integer))
  (returns (position :type "Vector Structure") (tangent :type "Vector Structure"))
  (bind _spline (`self.Spline`))
  (bind _sectionlength (`self.sectionLength`))
  (bind _returnvalue (* index _sectionlength))
  (return (`SplineComponent.GetLocationAtDistanceAlongSpline` _spline _returnvalue "Local") (`KismetMathLibrary.ClampVectorSize` (`SplineComponent.GetTangentAtDistanceAlongSpline` _spline _returnvalue "Local") 0.0 _sectionlength)))

(fn `PlaceBuild`
  (`parent.PlaceBuild`)
  (bind _keys (`BlueprintMapLibrary.Map_Keys` (`BuildableSplineComponent.SplineMeshComps` (`self.BuildableSpline`))))
  (for _array_element _keys
    (`PrimitiveComponent.SetMaterial` _array_element 0 "/Engine/EngineMaterials/DefaultMaterial.DefaultMaterial")
    (`PrimitiveComponent.SetMaterial` _array_element 1 (`self.MI_ConveyorBelt`))))

(fn `RotateBuild`
  (params (rotationInput :type "Float (double-precision)"))
  (if (`self.isStartLocked`)
    (`self.RotateBuild` (`self.endSupport`) rotationInput)
    (else
      (`self.RotateBuild` (`self.startSupport`) rotationInput))))

(fn `UserConstructionScript`
  (`parent.UserConstructionScript`)
  (bind _returnvalue (`KismetMaterialLibrary.CreateDynamicMaterialInstance` "/Game/Core/Assets/Materials/M_ConveyorBelt.M_ConveyorBelt" "MI_ConveyorBelt"))
  (set `self.MI_ConveyorBelt` _returnvalue))