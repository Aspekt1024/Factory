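; BP_ItemCombiner is a buildable with two item inputs and one output.
; On BeginPlay it creates attach points at its three marker components and sets their directions.
; It accepts every item, destroys it on receipt and prints a running count.
; No combining or output logic is present, so nothing is sent through the output point.
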(event `self.ReceiveBeginPlay`
  (`parent.ReceiveBeginPlay`)
  (bind _attachpoint (`self.Create AttachPoint` (`SceneComponent.K2_GetComponentToWorld` (`self.AttachPosInput1`))))
  (bind _output_get (set `self.AttachPoint_In1` _attachpoint))
  (`AttachPoint.SetDirection` _output_get "Input")
  (bind _attachpoint_2 (`self.Create AttachPoint` (`SceneComponent.K2_GetComponentToWorld` (`self.AttachPosInput2`))))
  (bind _output_get_2 (set `self.AttachPoint_In2` _attachpoint_2))
  (`AttachPoint.SetDirection` _output_get_2 "Input")
  (bind _attachpoint_3 (`self.Create AttachPoint` (`SceneComponent.K2_GetComponentToWorld` (`self.AttachPosOutput`))))
  (bind _output_get_3 (set `self.AttachPoint_Out` _attachpoint_3))
  (`AttachPoint.SetDirection` _output_get_3 "Output"))

(event `self.OnItemReceived`
  (params (AttachPoint :type "AttachPoint Object Reference") (Item :type "Item Object Reference"))
  (`self.K2_DestroyActor` Item)
  (bind _output_get (set `self.NumItems` (+ (`self.NumItems`) 1)))
  (`KismetSystemLibrary.PrintString` (`KismetStringLibrary.Conv_IntToString` _output_get)))

(fn `CanReceiveItem`
  (params (Item :type "Item Object Reference"))
  (returns (ReturnValue :type Boolean))
  (return true))

(fn `UserConstructionScript`
  (`parent.UserConstructionScript`))