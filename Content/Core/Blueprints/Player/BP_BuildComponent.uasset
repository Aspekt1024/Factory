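; Player build component that spawns, moves, rotates, places and deconstructs BP_Buildable actors such as conveyors and supports.
; Spawning starts at a camera-trace hit, and a looping timer updates the position while the buildable handles its own multi-step progress and cancel.
; Deconstruct mode shows the crosshair and uses a timed trace to highlight targets with a hologram material.
; Active timer handles act as mode state, routing Action and Cancel to build or deconstruct.
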(event `Action`
  ;[0.01447 0.1467 0.1962] Build Events
  (if (`KismetSystemLibrary.K2_IsValidTimerHandle` (`self.moveBuildTimer`))
    (`self.ProgressCurrentBuildable`)
    (else
      (`self.DeconstructSelectedItem`))))

(event `Cancel`
  ;[0.01447 0.1467 0.1962] Build Events
  (if (`KismetSystemLibrary.K2_IsValidTimerHandle` (`self.moveBuildTimer`))
    (`self.CancelCurrentBuildable`)
    (else
      (`self.CancelDeconstruct`))))

(event `RotateCurrentBuildable`
  (params (rotationInput :type "Float (double-precision)"))
  ;[0.01447 0.1467 0.1962] Build Events
  (bind _itemtobuild (`self.itemToBuild`)
    (:`then`
      (`/Game/Core/Blueprints/Buildables/BP_Buildable.RotateBuild` _itemtobuild rotationInput))
    (:`else`)))

(event `SpawnBuildable`
  (params (buildableType :type "/Game/Core/Blueprints/Buildables/BP_Buildable Class Reference"))
  (bind (_hitresult_out _ishit_out) (`PlayerSubsystem.LineTraceFromCamera` (subsystem `PlayerSubsystem`) "ECC_WorldStatic"))
  ;[0.01447 0.1467 0.1962] Buildable Spawn and Location Update
  (`self.CancelBuildCompletely`)
  (`self.CancelDeconstruct`)
  (if _ishit_out
    (bind _returnvalue (`|SpawnActorFromClass` buildableType (`KismetMathLibrary.MakeTransform` (`.Location` (`GameplayStatics.BreakHitResult` _hitresult_out))) "Undefined" "MultiplyWithRoot" null null))
    (set `self.itemToBuild` _returnvalue)
    (bind _returnvalue_2 (`KismetSystemLibrary.K2_SetTimerDelegate` (delegate `UpdateBuildPos`) (`self.moveInterval`) true))
    (set `self.moveBuildTimer` _returnvalue_2)))

(event `UpdateBuildPos`
  ;[0.01447 0.1467 0.1962] Buildable Spawn and Location Update
  (bind _itemtobuild (`self.itemToBuild`)
    (:`then`
      (`/Game/Core/Blueprints/Buildables/BP_Buildable.UpdateBuildPos` _itemtobuild))
    (:`else`
      (`self.ClearItemToBuild`))))

(event `EnableDeconstructMode`
  ;[0.01447 0.1467 0.1962] Deconstruct
  (if (not (`KismetSystemLibrary.K2_IsValidTimerHandle` (`self.deconstructTimer`)))
    (`self.CancelBuildCompletely`)
    (`/Game/Core/UI/WBP_HUD.SetCrosshairEnabled` (`self.HUD`) true)
    (bind _returnvalue (`KismetSystemLibrary.K2_SetTimerDelegate` (delegate `DeconstructLoop`) (`self.deconstructInterval`) true))
    (set `self.deconstructTimer` _returnvalue)))

(event `DeconstructLoop`
  (bind (_hitresult_out _ishit_out) (`PlayerSubsystem.LineTraceFromCamera` (subsystem `PlayerSubsystem`) "ECC_GameTraceChannel3"))
  ;[0.01447 0.1467 0.1962] Deconstruct
  (if _ishit_out
    (bind _asbp_buildable (cast `/Game/Core/Blueprints/Buildables/BP_Buildable` (`.HitActor` (`GameplayStatics.BreakHitResult` _hitresult_out)))
      (:`then`
        (bind _output_get (set `self.itemToDeconstruct` _asbp_buildable))
        (`/Game/Core/Blueprints/Buildables/BP_Buildable.SetAllMaterials` _output_get "/Game/Core/Assets/Materials/MI_HologramDestruct.MI_HologramDestruct" false))
      (:`CastFailed`
        (`self.ClearItemToDeconstruct` :!label _label)))
    (else
      (goto _label))))

(event `Object1`
  (`self.SpawnBuildable` "/Game/Core/Blueprints/Buildables/BP_Buildable_ConveyorSupport.BP_Buildable_ConveyorSupport_C"))

(event `Object2`
  (`self.SpawnBuildable` "/Game/Core/Blueprints/Buildables/BP_Buildable_Conveyor.BP_Buildable_Conveyor_C"))

(event `Object3`
  ;[1 1 1] This is not linked to Factory Character input
  (`self.SpawnBuildable` "/Game/Core/Blueprints/Buildables/BP_Buildable_ConveyorSupport.BP_Buildable_ConveyorSupport_C"))

(fn `CancelBuildCompletely`
  (locals (isComplete :type Boolean) (loopCount :type Integer) (maxCancelCount :type Integer :default 10))
  (set `local.isComplete` false)
  (while (not (`local.isComplete`))
    (bind _iscomplete (`self.CancelCurrentBuildable`))
    (if _iscomplete
      (set `local.isComplete` true)
      (else
        (bind _output_get (set `local.loopCount` (+ (`local.loopCount`) 1)))
        (if (>= _output_get (`local.maxCancelCount`))
          (`KismetSystemLibrary.PrintString` "Cancel Buildable never resolved!!" true true (struct :`R` 1.0 :`A` 1.0))
          (set `local.isComplete` true))))))

(fn `CancelCurrentBuildable`
  (returns (isComplete :type Boolean))
  (bind _itemtobuild (`self.itemToBuild`)
    (:`then`
      (bind _iscomplete (`/Game/Core/Blueprints/Buildables/BP_Buildable.CancelBuild` _itemtobuild))
      (if _iscomplete
        (set `self.itemToBuild` null)
        (`self.ClearItemToBuild`)
        (return true)
        (else
          (return false))))
    (:`else`
      (return true))))

(fn `CancelDeconstruct`
  (if (`KismetSystemLibrary.K2_IsValidTimerHandle` (`self.deconstructTimer`))
    (`KismetSystemLibrary.K2_ClearAndInvalidateTimerHandle` (`self.deconstructTimer`)))
  (`/Game/Core/UI/WBP_HUD.SetCrosshairEnabled` (`self.HUD`) false)
  (`self.ClearItemToDeconstruct`))

(fn `ClearItemToBuild`
  (bind _movebuildtimer (`self.moveBuildTimer`))
  (bind _itemtobuild (`self.itemToBuild`)
    (:`then`
      (`Actor.K2_DestroyActor` _itemtobuild))
    (:`else`
      _))
  (set `self.itemToBuild` null)
  (if (`KismetSystemLibrary.K2_IsValidTimerHandle` _movebuildtimer)
    (`KismetSystemLibrary.K2_ClearAndInvalidateTimerHandle` _movebuildtimer)))

(fn `ClearItemToDeconstruct`
  (bind _itemtodeconstruct (`self.itemToDeconstruct`)
    (:`then`
      (`/Game/Core/Blueprints/Buildables/BP_Buildable.SetAllMaterials` _itemtodeconstruct null true)
      (set `self.itemToDeconstruct` null))
    (:`else`)))

(fn `ClearMoveBuildTimer`
  (bind _movebuildtimer (`self.moveBuildTimer`))
  (if (`KismetSystemLibrary.K2_IsValidTimerHandle` _movebuildtimer)
    (`KismetSystemLibrary.K2_ClearAndInvalidateTimerHandle` _movebuildtimer)
    (set `self.moveBuildTimer` (struct))))

(fn `DeconstructSelectedItem`
  (bind _itemtodeconstruct (`self.itemToDeconstruct`)
    (:`then`
      (`/Game/Core/Blueprints/Buildables/BP_Buildable.Deconstruct` _itemtodeconstruct))
    (:`else`)))

(fn `Init`
  (params (HUD :type "/Game/Core/UI/WBP_HUD Object Reference"))
  (set `self.HUD` HUD))

(fn `PlaceBuildable`)

(fn `ProgressCurrentBuildable`
  (bind _itemtobuild (`self.itemToBuild`)
    (:`then`
      (bind _iscomplete (`/Game/Core/Blueprints/Buildables/BP_Buildable.ProgressBuild` _itemtobuild))
      (if _iscomplete
        (set `self.itemToBuild` null)
        (`self.ClearItemToBuild`)))
    (:`else`)))