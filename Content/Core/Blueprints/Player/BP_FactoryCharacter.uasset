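; Player character for a factory-building game that lets the player place, rotate, cancel and deconstruct buildables.
; On BeginPlay it initializes the PlayerSubsystem with itself and adds the gameplay Enhanced Input mapping context to the first player controller.
; Input actions forward straight to BuildComponent, including scroll for rotation and two object hotkeys, so the character holds no build logic of its own.
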(event `self.ReceiveBeginPlay`
  (`PlayerSubsystem.InitializeSubsystem` (subsystem `PlayerSubsystem`) self)
  (`self.SetupInput`))

(event `SetupInput`
  ;[0.01447 0.1467 0.1962] Setup Input
  (`EnhancedInputSubsystemInterface.AddMappingContext` (pcsubsystem `EnhancedInputLocalPlayerSubsystem` (`GameplayStatics.GetPlayerController` 0)) "/Game/Core/Blueprints/Inputs/IMC_Gameplay.IMC_Gameplay" 0 (struct)))

(event `EnhancedInput|/Game/Core/Blueprints/Inputs/IA_Confirm`
  (params (ActionValue :type Boolean) (ElapsedSeconds :type "Float (double-precision)") (TriggeredSeconds :type "Float (double-precision)") (InputAction :type "InputAction Object Reference" :default "/Game/Core/Blueprints/Inputs/IA_Confirm.IA_Confirm"))
  ;[0.01447 0.1467 0.1962] Building
  (:`Started`
    (`/Game/Core/Blueprints/Player/BP_BuildComponent.Build` (`self.BuildComponent`))))

(event `EnhancedInput|/Game/Core/Blueprints/Inputs/IA_Deconstruct`
  (params (ActionValue :type Boolean) (ElapsedSeconds :type "Float (double-precision)") (TriggeredSeconds :type "Float (double-precision)") (InputAction :type "InputAction Object Reference" :default "/Game/Core/Blueprints/Inputs/IA_Deconstruct.IA_Deconstruct"))
  ;[0.01447 0.1467 0.1962] Building
  (:`Started`
    (`/Game/Core/Blueprints/Player/BP_BuildComponent.Deconstruct` (`self.BuildComponent`))))

(event `EnhancedInput|/Game/Core/Blueprints/Inputs/IA_Scroll`
  (params (ActionValue :type "Float (double-precision)") (ElapsedSeconds :type "Float (double-precision)") (TriggeredSeconds :type "Float (double-precision)") (InputAction :type "InputAction Object Reference" :default "/Game/Core/Blueprints/Inputs/IA_Scroll.IA_Scroll"))
  ;[0.01447 0.1467 0.1962] Building
  (:`Started`
    (`/Game/Core/Blueprints/Player/BP_BuildComponent.RotateCurrentBuildable` (`self.BuildComponent`) ActionValue)))

(event `EnhancedInput|/Game/Core/Blueprints/Inputs/IA_Cancel`
  (params (ActionValue :type Boolean) (ElapsedSeconds :type "Float (double-precision)") (TriggeredSeconds :type "Float (double-precision)") (InputAction :type "InputAction Object Reference" :default "/Game/Core/Blueprints/Inputs/IA_Cancel.IA_Cancel"))
  ;[0.01447 0.1467 0.1962] Building
  (:`Started`
    (`/Game/Core/Blueprints/Player/BP_BuildComponent.CancelCurrentBuildable` (`self.BuildComponent`))))

(event `EnhancedInput|/Game/Core/Blueprints/Inputs/IA_Object1`
  (params (ActionValue :type Boolean) (ElapsedSeconds :type "Float (double-precision)") (TriggeredSeconds :type "Float (double-precision)") (InputAction :type "InputAction Object Reference" :default "/Game/Core/Blueprints/Inputs/IA_Object1.IA_Object1"))
  ;[0.01447 0.1467 0.1962] Building
  ;;[0.01447 0.1467 0.1962] Objects
  (:`Started`
    (`/Game/Core/Blueprints/Player/BP_BuildComponent.Object1` (`self.BuildComponent`))))

(event `EnhancedInput|/Game/Core/Blueprints/Inputs/IA_Object2`
  (params (ActionValue :type Boolean) (ElapsedSeconds :type "Float (double-precision)") (TriggeredSeconds :type "Float (double-precision)") (InputAction :type "InputAction Object Reference" :default "/Game/Core/Blueprints/Inputs/IA_Object2.IA_Object2"))
  ;[0.01447 0.1467 0.1962] Building
  ;;[0.01447 0.1467 0.1962] Objects
  (:`Started`
    (`/Game/Core/Blueprints/Player/BP_BuildComponent.Object2` (`self.BuildComponent`))))

(fn `UserConstructionScript`
  (`parent.UserConstructionScript`))